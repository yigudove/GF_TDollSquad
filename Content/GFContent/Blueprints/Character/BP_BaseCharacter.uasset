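; BP_BaseCharacter is a character Blueprint that drives an overhead debug text widget.
; BeginPlay casts the OverheadInfo component's user widget to OverheadWidget and fetches its controller name block.
; Each Tick writes LastTraceItem's object name to the trace item block, or "NULL" when invalid, in which case it also writes the character's display name to the controller block.
; A ShowPlayerNetRole call remains unconnected.
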(event `self.ReceiveBeginPlay`
  (bind _asoverhead_widget (cast `OverheadWidget` (`WidgetComponent.GetUserWidgetObject` (`self.OverheadInfo`))))
  (bind _returnvalue (`OverheadWidget.GetControllerNameBlock` _asoverhead_widget)))

(event `self.ReceiveTick`
  (params (DeltaSeconds :type "Float (single-precision)"))
  (bind _returnvalue (`OverheadWidget.GetLastTraceItemNameBlock` (stale `self.ReceiveBeginPlay` _asoverhead_widget)))
  (if (`KismetSystemLibrary.IsValid` (`self.LastTraceItem`))
    (`OverheadWidget.SetTextBlock` (stale `self.ReceiveBeginPlay` _asoverhead_widget) _returnvalue (`KismetSystemLibrary.GetObjectName` (`self.LastTraceItem`)))
    (else
      (bind _output_get (set `self.NewVar` "NULL"))
      (`OverheadWidget.SetTextBlock` (stale `self.ReceiveBeginPlay` _asoverhead_widget) _returnvalue _output_get)
      (`OverheadWidget.SetTextBlock` (stale `self.ReceiveBeginPlay` _asoverhead_widget) (stale `self.ReceiveBeginPlay` _returnvalue) (`KismetSystemLibrary.GetDisplayName` self)))))

(fn `UserConstructionScript`)